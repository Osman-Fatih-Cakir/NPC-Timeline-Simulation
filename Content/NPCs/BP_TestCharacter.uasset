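; Test NPC character that jogs endlessly between random nearby navmesh points.
; On BeginPlay it plays a looping jogging animation directly on the skeletal mesh, then picks a random navigable point within a fixed radius of its current location.
; It snaps its rotation toward that point and uses AI Move To to travel there.
; Each successful arrival picks the next point; a failed move is unhandled, so the wandering stops.
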(event EventBeginPlay
  (bind _defaultsceneroot (Variables|Default|GetDefaultSceneRoot))
  (bind _defaultsceneroot_2 (Variables|Default|GetDefaultSceneRoot))
  (bind _returnvalue (Transformation|GetWorldLocation _defaultsceneroot_2))
  (bind _returnvalue_2 (Transformation|GetWorldLocation _defaultsceneroot))
  (Components|Animation|PlayAnimation (Variables|Default|GetSkeletalMesh) "/Game/Anims/Jogging/Jogging__1__Anim_mixamo_com.Jogging__1__Anim_mixamo_com" true)
  ;[1 1 1] move random loc
  (bind _randomlocation (Class|NavigationSystemV1|GetRandomLocationinNavigableRadius _returnvalue 5e+02 0 "/Script/NavigationSystem.RecastFilter_UseDefaultArea" :!label _label))
  (bind _output_get (Variables|Default|SetnextPosDirection (- _randomlocation _returnvalue)))
  (Class|KismetMathLibrary|VectorSet (Variables|Default|GetnextPosDirection) (.X (Math|Vector|BreakVector _output_get)) (.Y (Math|Vector|BreakVector _output_get)) 0.0)
  (Transformation|SetActorRotation (Math|Rotator|FindLookatRotation _returnvalue_2 (+ _returnvalue_2 (Variables|Default|GetnextPosDirection))))
  (AI|AIMoveTo self _randomlocation 0 1e+01 false
    (:OnSuccess
      (goto _label))))

(fn ConstructionScript)